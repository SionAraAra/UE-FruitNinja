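; BP_Sword is a grabbable VR sword that slices fruit and bombs for points.
; Grabbing or dropping it hides or shows that hand through a message to the motion controller's owner, avoiding a hard VR pawn reference.
; Mesh overlaps run a cast chain over bomb, pomegranate, pear, orange and watermelon, adding the match's Points to Player's Score and destroying it.
; A katana sound plays on every overlap.
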(event OnGrabbed(GrabComponentSnap)
  (bind _grabcomponentsnap (Variables|Default|GetGrabComponentSnap))
  (Class|BPIPawnAnim|HideUnhideHand(Message) (Components|GetOwner (Variables|/Game/VRTemplate/Blueprints/GrabComponent.GrabComponent_C|GetMotionControllerRef _grabcomponentsnap)) true (Utilities|Enum|Equal(Enum) (Default|GetHeldbyHand _grabcomponentsnap) "Right")))

(event OnDropped(GrabComponentSnap)
  (bind _grabcomponentsnap (Variables|Default|GetGrabComponentSnap))
  (Class|BPIPawnAnim|HideUnhideHand(Message) (Components|GetOwner (Variables|/Game/VRTemplate/Blueprints/GrabComponent.GrabComponent_C|GetMotionControllerRef _grabcomponentsnap)) false (Utilities|Enum|Equal(Enum) (Default|GetHeldbyHand _grabcomponentsnap) "Right")))

(event OnComponentBeginOverlap(StaticMesh)
  (params (OverlappedComponent :type Primitive%20Component%20Object%20Reference) (OtherActor :type Actor%20Object%20Reference) (OtherComp :type Primitive%20Component%20Object%20Reference) (OtherBodyIndex :type Integer) (bFromSweep :type Boolean) (SweepResult :type Hit%20Result%20Structure%20%28by%20ref%29))
  (CallFunction|CasttoFruit OtherActor)
  (Audio|PlaySound2D "/Game/OwnContent/katana.katana" 1.0 1.0 0.0 0 0))

(event Collision|EventActorBeginOverlap
  (params (OtherActor :type Actor%20Object%20Reference)))

(event EventTick
  (params (DeltaSeconds :type Float%20%28single-precision%29)))

(fn ConstructionScript)

(fn CasttoFruit
  (params (Actor :type Actor%20Object%20Reference))
  (bind _asbp_bomb (Utilities|Casting|CastToBP_BOMB Actor)
    (:then
      (CallFunction|AddScore (Variables|/Game/OwnContent/Fruit/BP_BOMB.BP_BOMB_C|GetPoints _asbp_bomb))
      (Actor|DestroyActor _asbp_bomb))
    (:CastFailed
      (bind _asbp_pomegranate (Utilities|Casting|CastToBP_Pomegranate Actor)
        (:then
          (CallFunction|AddScore (Variables|/Game/OwnContent/Fruit/BP_Pomegranate.BP_Pomegranate_C|GetPoints _asbp_pomegranate))
          (Actor|DestroyActor _asbp_pomegranate))
        (:CastFailed
          (bind _asbp_pear (Utilities|Casting|CastToBP_Pear Actor)
            (:then
              (CallFunction|AddScore (Variables|/Game/OwnContent/Fruit/BP_Pear.BP_Pear_C|GetPoints _asbp_pear))
              (Actor|DestroyActor _asbp_pear))
            (:CastFailed
              (bind _asbp_orange (Utilities|Casting|CastToBP_Orange Actor)
                (:then
                  (CallFunction|AddScore (Variables|/Game/OwnContent/Fruit/BP_Orange.BP_Orange_C|GetPoints _asbp_orange))
                  (Actor|DestroyActor _asbp_orange))
                (:CastFailed
                  (bind _asbp_watermelon (Utilities|Casting|CastToBP_Watermelon Actor))
                  (CallFunction|AddScore (Variables|/Game/OwnContent/Fruit/BP_Watermelon.BP_Watermelon_C|GetPoints _asbp_watermelon))
                  (Actor|DestroyActor _asbp_watermelon))))))))))

(fn AddScore
  (params (points :type Integer))
  (bind _player (Variables|Default|GetPlayer))
  (Variables|/Game/VRTemplate/Blueprints/VRPawn.VRPawn_C|SetScore _player (+ points (Variables|/Game/VRTemplate/Blueprints/VRPawn.VRPawn_C|GetScore _player))))