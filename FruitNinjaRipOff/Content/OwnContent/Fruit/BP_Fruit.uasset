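; BP_Fruit is a spawner actor that periodically spawns an orange, bomb, pomegranate, pear or watermelon.
; A Delay on Tick paces spawning by SpawnInterval, and a chain of random-integer branches picks the class.
; Each branch rolls anew, so odds favor earlier entries and some cycles spawn nothing.
; Spawns use the actor's own transform, with X offset randomly between MinRange and MaxRange.
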(event EventTick
  (params (DeltaSeconds :type Float%20%28single-precision%29))
  (bind _returnvalue (Transformation|GetActorTransform))
  (bind _returnvalue_2 (Transformation|GetActorTransform))
  (bind _returnvalue_3 (Transformation|GetActorTransform))
  (bind _returnvalue_4 (Transformation|GetActorTransform))
  (bind _returnvalue_5 (Transformation|GetActorTransform))
  (bind _returnvalue_6 (Math|Random|RandomIntegerinRange 0 4))
  (Utilities|FlowControl|Delay (Variables|Default|GetSpawnInterval))
  (if (== _returnvalue_6 0)
    (Game|SpawnActorfromClass "/Game/OwnContent/Fruit/BP_Orange.BP_Orange_C" (Math|Transform|MakeTransform (Math|Vector|MakeVector (+ (.x (.location _returnvalue_2)) (Math|Random|RandomFloatinRange (Variables|Default|GetMinRange) (Variables|Default|GetMaxRange))) (.y (.location _returnvalue_2)) (.z (.location _returnvalue_2))) (.rotation _returnvalue_2) (.scale _returnvalue_2)) "Undefined" "MultiplyWithRoot" 0 0)
    (elif (== _returnvalue_6 1)
      (Game|SpawnActorfromClass "/Game/OwnContent/Fruit/BP_BOMB.BP_BOMB_C" (Math|Transform|MakeTransform (Math|Vector|MakeVector (+ (.x (.location _returnvalue)) (Math|Random|RandomFloatinRange (Variables|Default|GetMinRange) (Variables|Default|GetMaxRange))) (.y (.location _returnvalue)) (.z (.location _returnvalue))) (.rotation _returnvalue) (.scale _returnvalue)) "Undefined" "MultiplyWithRoot" 0 0)
      (elif (== _returnvalue_6 2)
        (Game|SpawnActorfromClass "/Game/OwnContent/Fruit/BP_Pomegranate.BP_Pomegranate_C" (Math|Transform|MakeTransform (Math|Vector|MakeVector (+ (.x (.location _returnvalue_3)) (Math|Random|RandomFloatinRange (Variables|Default|GetMinRange) (Variables|Default|GetMaxRange))) (.y (.location _returnvalue_3)) (.z (.location _returnvalue_3))) (.rotation _returnvalue_3) (.scale _returnvalue_3)) "Undefined" "MultiplyWithRoot" 0 0)
        (elif (== _returnvalue_6 3)
          (Game|SpawnActorfromClass "/Game/OwnContent/Fruit/BP_Pear.BP_Pear_C" (Math|Transform|MakeTransform (Math|Vector|MakeVector (+ (.x (.location _returnvalue_4)) (Math|Random|RandomFloatinRange (Variables|Default|GetMinRange) (Variables|Default|GetMaxRange))) (.y (.location _returnvalue_4)) (.z (.location _returnvalue_4))) (.rotation _returnvalue_4) (.scale _returnvalue_4)) "Undefined" "MultiplyWithRoot" 0 0)
          (elif (== _returnvalue_6 4)
            (Game|SpawnActorfromClass "/Game/OwnContent/Fruit/BP_Watermelon.BP_Watermelon_C" (Math|Transform|MakeTransform (Math|Vector|MakeVector (+ (.x (.location _returnvalue_5)) (Math|Random|RandomFloatinRange (Variables|Default|GetMinRange) (Variables|Default|GetMaxRange))) (.y (.location _returnvalue_5)) (.z (.location _returnvalue_5))) (.rotation _returnvalue_5) (.scale _returnvalue_5)) "Undefined" "MultiplyWithRoot" 0 0)))))))

(fn ConstructionScript)